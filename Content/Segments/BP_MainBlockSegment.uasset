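; BP_MainBlockSegment is a block segment actor that moves between its root position and a spot 100 units above it.
; It records its spawn location on BeginPlay, then each Tick picks the root as target when IsBlockEnabled, or the raised spot otherwise.
; When off target, it captures its start position and a timeline drives a circular in-out eased transform lerp, gated by a TweenFinished flag.
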(event `self.ReceiveBeginPlay`
  (set `self.fvRootPosition` (`self.K2_GetActorLocation`))
  (bind _asgameprodv_super_land_game_mode_base (cast `GAMEPRODV_SuperLandGameModeBase` (`GameplayStatics.GetGameMode`))))

(event `self.ReceiveTick`
  (params (DeltaSeconds :type "Float (single-precision)"))
  (if (`self.bIsBlockEnabled`)
    (set `self.fvTargetPosition` (`self.fvRootPosition`))
    (else
      (set `self.fvTargetPosition` (`KismetMathLibrary.MakeVector` (.x (`self.fvRootPosition`)) (.y (`self.fvRootPosition`)) (- (.z (`self.fvRootPosition`)) -100.0)))))
  (if (== (`self.K2_GetActorLocation`) (`self.fvTargetPosition`) :`ErrorTolerance` 1.0)
    _
    (elif (`self.bTweenFinished`)
      (set `self.StartPosition` (`self.K2_GetActorLocation`))
      (set `self.bTweenFinished` false)
      (elif (not (`self.bTweenFinished`))
        (bind (_direction _newtrack_2) (`Timeline|Timeline_0`)
          (:`Update`
            (`self.K2_SetActorTransform` (`KismetMathLibrary.TLerp` (`KismetMathLibrary.Conv_VectorToTransform` (`self.StartPosition`)) (`KismetMathLibrary.Conv_VectorToTransform` (`self.fvTargetPosition`)) (`|EaseFunction` "CircularInOut" _newtrack_2 0.0 1.0))))
          (:`Finished`
            (set `self.bTweenFinished` true)))))))

(fn `NewFunction_0`
  (returns (NewParam :type Boolean)))

(fn `UserConstructionScript`)